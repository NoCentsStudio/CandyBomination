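; Ladder actor that lets a PaperCharacter_Prototype climb while it overlaps the ladder's Box.
; The construction script stacks collision-free rung sprites at fixed spacing to span the LadderBottom-to-LadderTop height, then scales and offsets the Box from that height.
; Box overlap sets the character's CanClimb flag; leaving clears it and calls ClimbingEnd on the character.
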(event OnComponentBeginOverlap(Box)
  (params (OverlappedComponent :type Primitive%20Component%20Object%20Reference) (OtherActor :type Actor%20Object%20Reference) (OtherComp :type Primitive%20Component%20Object%20Reference) (OtherBodyIndex :type Integer) (bFromSweep :type Boolean) (SweepResult :type Hit%20Result%20Structure%20%28by%20ref%29))
  (bind _aspaper_character_prototype (Utilities|Casting|CastToPaperCharacter_Prototype OtherActor))
  (Variables|/Game/Blueprint/PaperCharacter_Prototype.PaperCharacter_Prototype_C|SetCanClimb _aspaper_character_prototype true))

(event OnComponentEndOverlap(Box)
  (params (OverlappedComponent :type Primitive%20Component%20Object%20Reference) (OtherActor :type Actor%20Object%20Reference) (OtherComp :type Primitive%20Component%20Object%20Reference) (OtherBodyIndex :type Integer))
  (bind _aspaper_character_prototype (Utilities|Casting|CastToPaperCharacter_Prototype OtherActor))
  (Variables|/Game/Blueprint/PaperCharacter_Prototype.PaperCharacter_Prototype_C|SetCanClimb _aspaper_character_prototype false)
  (Default|ClimbingEnd _aspaper_character_prototype))

(fn ConstructionScript
  (bind _ladderbottom (Variables|Default|GetLadderBottom))
  (bind _laddertop (Variables|Default|GetLadderTop))
  (bind _box (Variables|Default|GetBox))
  (bind _returnvalue (- _laddertop _ladderbottom))
  (bind _returnvalue_2 (/ (.z _returnvalue) 2.0))
  ;[1 1 1] Ladder Collision&Sprite Adjustement
  (Variables|Default|SetRungOffset 27.6)
  (for _index (range 0 (Math|Float|Truncate (/ (.z _returnvalue) (Variables|Default|GetRungOffset))))
    (bind _returnvalue_3 (AddComponent|AddPaperSpriteComponent false (Math|Transform|MakeTransform (Math|Vector|MakeVector 0.0 0.0 (* _index (Variables|Default|GetRungOffset))) "0, 0, 0" "0.750000,1,0.800000")))
    (Rendering|Components|Sprite|SetSprite _returnvalue_3 (Variables|Default|GetLadderSprite))
    (Collision|SetCollisionEnabled _returnvalue_3 "NoCollision"))
  (Transformation|SetRelativeScale3D _box (Math|Vector|MakeVector 5.0 1.0 _returnvalue_2))
  (Transformation|AddRelativeLocation _box (Math|Vector|MakeVector 0.0 0.0 _returnvalue_2) false false))