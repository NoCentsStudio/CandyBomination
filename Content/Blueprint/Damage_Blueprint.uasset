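; Damage_Blueprint is a trigger actor that lowers a Health value when the Paper2D prototype character overlaps its Box.
; Begin overlap casts to PaperCharacter_Prototype and subtracts one from Health while it is above zero; end overlap only performs the cast.
; The construction script adds a non-colliding Paper sprite through a single-iteration loop, leaving detection to the Box.
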(event OnComponentBeginOverlap(Box)
  (params (OverlappedComponent :type Primitive%20Component%20Object%20Reference) (OtherActor :type Actor%20Object%20Reference) (OtherComp :type Primitive%20Component%20Object%20Reference) (OtherBodyIndex :type Integer) (bFromSweep :type Boolean) (SweepResult :type Hit%20Result%20Structure%20%28by%20ref%29))
  (Utilities|Casting|CastToPaperCharacter_Prototype OtherActor)
  (Math|Integer|CompareInt (Variables|Default|GetHealth)
    (:>
      (Variables|Default|SetHealth (- (Variables|Default|GetHealth) 1)))))

(event OnComponentEndOverlap(Box)
  (params (OverlappedComponent :type Primitive%20Component%20Object%20Reference) (OtherActor :type Actor%20Object%20Reference) (OtherComp :type Primitive%20Component%20Object%20Reference) (OtherBodyIndex :type Integer))
  (Utilities|Casting|CastToPaperCharacter_Prototype OtherActor))

(fn ConstructionScript
  (for _index (range 0 0)
    (bind _returnvalue (AddComponent|AddPaperSpriteComponent false))
    (Rendering|Components|Sprite|SetSprite _returnvalue "/Game/Sprites/Construction_Texture_Sprite_0.Construction_Texture_Sprite_0")
    (Collision|SetCollisionEnabled _returnvalue "NoCollision")))